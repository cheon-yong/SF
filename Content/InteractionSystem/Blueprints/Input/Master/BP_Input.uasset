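; BP_Input is the master Blueprint for inputs in the interaction system, holding an on/off State and a list of Connections.
; Set State On and Set State Off update State, then call BeginInteract or EndInteract on every connection, passing along the interacting pawn.
; Update Children, Get Fracture Bool, Get Item Type and Get Mesh are stubs that do nothing or return defaults.
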(fn ConstructionScript)

(fn UpdateChildren)

(fn SetStateon
  (params (Interact%20Pawn :type Actor%20Object%20Reference))
  (Variables|Runtime|SetState true)
  (for _array_element (Variables|Data|GetConnections)
    (Class|InteractActor|BeginInteract _array_element Interact%20Pawn)))

(fn SetStateOff
  (params (Interact%20Pawn :type Actor%20Object%20Reference))
  (Variables|Runtime|SetState false)
  (for _array_element (Variables|Data|GetConnections)
    (Class|InteractActor|EndInteract _array_element Interact%20Pawn)))

(fn GetFractureBool
  (return false))

(fn GetItemType
  (return "NewEnumerator0"))

(fn GetMesh
  (return 0))