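; BP_Button_Bricks is an interactable push button that triggers its linked InteractActors.
; When State is on, the server plays the player's push montage, then a delayed timeline depresses the top.
; At the press point it plays a sound, switches off State and light material, disables collision, and forwards the interaction.
; Multi_PushButtonEffect duplicates this press sequence with authority-only forwarding, and SyncInputState lets external callers set State.
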(event Custom|Multi_PushButtonEffect
  (params (InteractPawn :type Actor%20Object%20Reference))
  (Utilities|FlowControl|Delay 0.5)
  (bind _alpha (Timeline|Timeline PlayFromStart)
    (:Update
      (Transformation|SetRelativeLocation (Variables|Default|GetSM_Button_Top) (Math|Vector|Lerp(Vector) "0, 0, 0" "0, 0,-5.000000" _alpha) false false))
    (:Button%20Press
      (Audio|Components|Audio|SetSound (Variables|Default|GetAudio) (Variables|Runtime|GetButtonSound))
      (Audio|Components|Audio|Play (Variables|Default|GetAudio) 0.0)
      (CallFunction|SetStateOff)
      (CallFunction|UpdateLight)
      (Collision|SetCollisionEnabled (Variables|Default|GetStaticMeshComponent) "NoCollision")
      (Networking|SwitchHasAuthority
        (:Authority
          (CallFunction|InteractOther InteractPawn))))))

(event EventBeginPlay
  (Networking|SwitchHasAuthority
    (:Authority
      (CallFunction|UpdateLight))))

(event EventSyncInputState
  (params (State :type Boolean))
  (Variables|Runtime|SetState State)
  (CallFunction|UpdateLight))

(event EventBeginInteract
  (params (InInteractPawn :type Actor%20Object%20Reference))
  (Networking|SwitchHasAuthority
    (:Authority
      (if (Variables|Runtime|GetState)
        (Class|SFPlayerCharacter|PlayAnimMontageandBlockMove (.AsSFPlayer%20Character (Utilities|Casting|CastToSFPlayerCharacter InInteractPawn)) (Variables|Runtime|GetButtonPushAnim) 1.0 "0.000000,0.000000,0.000000" "None")
        (Utilities|FlowControl|Delay 0.5)
        (bind _alpha (Timeline|Timeline_ButtonAnimation PlayFromStart)
          (:Update
            (Transformation|SetRelativeLocation (Variables|Default|GetSM_Button_Top) (Math|Vector|Lerp(Vector) "0, 0, 0" "0, 0,-5.000000" _alpha) false false))
          (:Button%20Press
            (Audio|Components|Audio|SetSound (Variables|Default|GetAudio) (Variables|Runtime|GetButtonSound))
            (Audio|Components|Audio|Play (Variables|Default|GetAudio) 0.0)
            (CallFunction|SetStateOff)
            (CallFunction|UpdateLight)
            (Collision|SetCollisionEnabled (Variables|Default|GetStaticMeshComponent) "NoCollision")
            (CallFunction|InteractOther InInteractPawn)))))))

(fn ConstructionScript)

(fn UpdateLight
  (Rendering|Material|SetMaterial (Variables|Default|GetSM_Button_Top) 0 (select (Variables|Runtime|GetState) "/Game/InteractionSystem/Assets/Materials/ProcGrid/MI_ProcGrid_OnLines.MI_ProcGrid_OnLines" "/Game/InteractionSystem/Assets/Materials/ProcGrid/MI_ProcGrid_OffLines.MI_ProcGrid_OffLines")))

(fn SyncState
  (for _array_element (Variables|Data|GetInput%20Sync)
    (Class|BPIInteraction|SyncInputState(Message) _array_element (Variables|Runtime|GetState))))

(fn SetStateon
  (Variables|Runtime|SetState true))

(fn SetStateOff
  (Variables|Runtime|SetState false))

(fn InteractOther
  (params (InteractPawn :type Actor%20Object%20Reference))
  (for _array_element (Variables|Data|GetInteractActors)
    (Class|InteractActor|BeginInteract _array_element InteractPawn)))

(fn GetFractureBool
  (return false))

(fn GetItemType
  (return "NewEnumerator0"))

(fn GetMesh
  (return 0))