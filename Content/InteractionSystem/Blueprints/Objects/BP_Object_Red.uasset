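; BP_Object_Red is a breakable item in the interaction system that shatters under projectile fire.
; On the server, mesh hits from SFProjectiles reduce HP, but only when the instigator of the projectile's owner is not locally controlled.
; At zero HP, SpawnFragments spawns short-lived, red-lined BP_Item fracture pieces inheriting the mesh velocity, then drops and destroys the object.
; The BreakItem event is left empty.
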(event OnComponentHit(Mesh)
  (params (HitComponent :type Primitive%20Component%20Object%20Reference) (OtherActor :type Actor%20Object%20Reference) (OtherComp :type Primitive%20Component%20Object%20Reference) (NormalImpulse :type Vector :default "0, 0, 0") (Hit :type Hit%20Result%20Structure%20%28by%20ref%29))
  (Networking|SwitchHasAuthority
    (:Authority
      (bind _assfprojectile (Utilities|Casting|CastToSFProjectile OtherActor))
      (if (not (Pawn|IsLocallyControlled (Variables|/Script/Engine.Actor|GetInstigator (Components|GetOwner _assfprojectile))))
        (bind _output_get (Variables|Default|SetHP (- (Variables|Default|GetHP) 1)))
        (if (<= _output_get 0)
          (Variables|Runtime|SetBroken true)
          (CallFunction|SpawnFragments))))))

(event EventBeginPlay
  (|CallParentFunction) ; This node is disabled and will not be called.\nDrag off pins to build functionality.
)

(event EventTick
  (params (DeltaSeconds :type Float%20%28single-precision%29))
  (|CallParentFunction DeltaSeconds) ; This node is disabled and will not be called.\nDrag off pins to build functionality.
)

(event EventBreakItem)

(fn ConstructionScript
  (|CallParentFunction))

(fn SpawnFragments
  (bind _mesh (Variables|Character|GetMesh))
  (for _array_element (Variables|Init|GetFragments)
    (bind _returnvalue (Game|SpawnActorfromClass "/Game/InteractionSystem/Blueprints/Items/Master/BP_Item.BP_Item_C" (Transformation|GetWorldTransform _mesh) "Undefined" "OverrideRootScale" 0 _array_element (Transformation|GetComponentVelocity _mesh) true 0))
    (Rendering|Material|SetMaterial (Variables|/Game/InteractionSystem/Blueprints/Items/Master/BP_Item.BP_Item_C|GetMesh _returnvalue) 0 "/Game/InteractionSystem/Assets/Materials/ProcGrid/MI_ProcGrid_RedLines.MI_ProcGrid_RedLines")
    (Actor|SetLifeSpan _returnvalue 3.0))
  (CallFunction|DropItem "0, 0, 0" true)
  (Actor|DestroyActor))